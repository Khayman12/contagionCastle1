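; Player 2's character Blueprint: a child class that sets its "Player2" row name and handles traps, slashing, crouching, curing and infection.
; Action events, with Multi and Server variants sharing the same logic, set Anim_france flags, spawn tripwire, attack or cure actors, and update item counts or HUD flags.
; While infected, Tick stops movement, shows text, then after a delay flags the HUD as turned.
; Overlapping an antidote-carrying BP_Player1 sets Cure.
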(event OnComponentBeginOverlap(infactArea)
  (params (OverlappedComponent :type Primitive%20Component%20Object%20Reference) (OtherActor :type Actor%20Object%20Reference) (OtherComp :type Primitive%20Component%20Object%20Reference) (OtherBodyIndex :type Integer) (bFromSweep :type Boolean) (SweepResult :type Hit%20Result%20Structure%20%28by%20ref%29))
  ;[1 1 1] cure
  (bind _asbp_player_1 (Utilities|Casting|CastToBP_Player1 OtherActor))
  (if (> (Variables|/Game/NewPlayers/BP_basePlayer.BP_basePlayer_C|GetAntidote _asbp_player_1) 0)
    (Variables|Default|SetCure true)))

(event Custom|startCrouch
  ;[1 1 1] crouch
  (bind _asanim_france (Utilities|Casting|CastToAnim_france (Components|SkeletalMesh|GetAnimInstance (Variables|Character|GetMesh))))
  (Variables|/Game/anim/Francesca/Animations/Anim_france.Anim_france_C|SetisCrouching _asanim_france true))

(event Custom|startCrouchMulti
  ;[1 1 1] crouch
  (bind _asanim_france (Utilities|Casting|CastToAnim_france (Components|SkeletalMesh|GetAnimInstance (Variables|Character|GetMesh))))
  (Variables|/Game/anim/Francesca/Animations/Anim_france.Anim_france_C|SetisCrouching _asanim_france true))

(event Custom|stopCrouchMulti
  ;[1 1 1] crouch
  (bind _asanim_france (Utilities|Casting|CastToAnim_france (Components|SkeletalMesh|GetAnimInstance (Variables|Character|GetMesh))))
  (Variables|/Game/anim/Francesca/Animations/Anim_france.Anim_france_C|SetisCrouching _asanim_france false))

(event Custom|stopCrouchSever
  ;[1 1 1] crouch
  (bind _asanim_france (Utilities|Casting|CastToAnim_france (Components|SkeletalMesh|GetAnimInstance (Variables|Character|GetMesh))))
  (Variables|/Game/anim/Francesca/Animations/Anim_france.Anim_france_C|SetisCrouching _asanim_france false))

(event Custom|startSetTrap
  ;[1 1 1] settrap
  (bind _asanim_france (Utilities|Casting|CastToAnim_france (Components|SkeletalMesh|GetAnimInstance (Variables|Character|GetMesh))))
  (Variables|/Game/anim/Francesca/Animations/Anim_france.Anim_france_C|SetcanSetTrap _asanim_france true)
  (Utilities|FlowControl|Delay 1.17)
  (Game|SpawnActorfromClass "/Game/NewPlayers/Abiltys/tripWire.tripWire_C" (Transformation|GetWorldTransform (Variables|Default|GetTripwireArrow)) "Undefined" 0 0)
  (bind _output_get (Variables|Default|SetTrip%20Wire (- (Variables|Default|GetTrip%20Wire) 1)))
  (if (<= _output_get 0)
    (bind _output_get_2 (Variables|/Game/NewPlayers/BP_basePlayer.BP_basePlayer_C|SetWB_IngameHUD self (Variables|Default|GetWb_InGameHUD)))
    (Variables|/Game/NewPlayers/widgets/WB_InGameHUD.WB_InGameHUD_C|SetcanSetTrap _output_get_2 false)))

(event Custom|stopSetTrap
  ;[1 1 1] settrap
  (Utilities|FlowControl|Delay 2.53)
  (bind _asanim_france (Utilities|Casting|CastToAnim_france (Components|SkeletalMesh|GetAnimInstance (Variables|Character|GetMesh))))
  (Variables|/Game/anim/Francesca/Animations/Anim_france.Anim_france_C|SetcanSetTrap _asanim_france false))

(event Custom|startSlashMulti
  ;[1 1 1] slahs
  (bind _asanim_france (Utilities|Casting|CastToAnim_france (Components|SkeletalMesh|GetAnimInstance (Variables|Character|GetMesh))))
  (Variables|/Game/anim/Francesca/Animations/Anim_france.Anim_france_C|SetcanSlash _asanim_france false)
  (Game|SpawnActorfromClass "/Game/NewPlayers/Abiltys/player1Attack.player1Attack_C" (Transformation|GetWorldTransform (Variables|Default|GetArrow2)) "Undefined" 0 0)
  (bind _output_get (Variables|/Game/NewPlayers/BP_basePlayer.BP_basePlayer_C|SetWB_IngameHUD self (Variables|Default|GetWb_InGameHUD)))
  (Variables|/Game/NewPlayers/widgets/WB_InGameHUD.WB_InGameHUD_C|SetcanMonsterAttack _output_get false))

(event Custom|stopSetTrapMulti
  ;[1 1 1] settrap
  (Utilities|FlowControl|Delay 2.53)
  (bind _asanim_france (Utilities|Casting|CastToAnim_france (Components|SkeletalMesh|GetAnimInstance (Variables|Character|GetMesh))))
  (Variables|/Game/anim/Francesca/Animations/Anim_france.Anim_france_C|SetcanSetTrap _asanim_france false))

(event Custom|stopSetTrapSever
  ;[1 1 1] settrap
  (Utilities|FlowControl|Delay 2.53)
  (bind _asanim_france (Utilities|Casting|CastToAnim_france (Components|SkeletalMesh|GetAnimInstance (Variables|Character|GetMesh))))
  (Variables|/Game/anim/Francesca/Animations/Anim_france.Anim_france_C|SetcanSetTrap _asanim_france false))

(event Custom|stopSlashMulti
  ;[1 1 1] slahs
  (Utilities|FlowControl|Delay 1.47)
  (bind _asanim_france (Utilities|Casting|CastToAnim_france (Components|SkeletalMesh|GetAnimInstance (Variables|Character|GetMesh))))
  (Variables|/Game/anim/Francesca/Animations/Anim_france.Anim_france_C|SetcanSlash _asanim_france false))

(event Custom|stopSlashSever
  ;[1 1 1] slahs
  (Utilities|FlowControl|Delay 1.47)
  (bind _asanim_france (Utilities|Casting|CastToAnim_france (Components|SkeletalMesh|GetAnimInstance (Variables|Character|GetMesh))))
  (Variables|/Game/anim/Francesca/Animations/Anim_france.Anim_france_C|SetcanSlash _asanim_france false))

(event Custom|startSetTrapMulti
  ;[1 1 1] settrap
  (bind _asanim_france (Utilities|Casting|CastToAnim_france (Components|SkeletalMesh|GetAnimInstance (Variables|Character|GetMesh))))
  (Variables|/Game/anim/Francesca/Animations/Anim_france.Anim_france_C|SetcanSetTrap _asanim_france true)
  (Utilities|FlowControl|Delay 1.17)
  (Game|SpawnActorfromClass "/Game/NewPlayers/Abiltys/tripWire.tripWire_C" (Transformation|GetWorldTransform (Variables|Default|GetTripwireArrow)) "Undefined" 0 0)
  (bind _output_get (Variables|Default|SetTrip%20Wire (- (Variables|Default|GetTrip%20Wire) 1)))
  (if (<= _output_get 0)
    (bind _output_get_2 (Variables|/Game/NewPlayers/BP_basePlayer.BP_basePlayer_C|SetWB_IngameHUD self (Variables|Default|GetWb_InGameHUD)))
    (Variables|/Game/NewPlayers/widgets/WB_InGameHUD.WB_InGameHUD_C|SetcanSetTrap _output_get_2 false)))

(event Custom|startSlashServer
  ;[1 1 1] slahs
  (bind _asanim_france (Utilities|Casting|CastToAnim_france (Components|SkeletalMesh|GetAnimInstance (Variables|Character|GetMesh))))
  (Variables|/Game/anim/Francesca/Animations/Anim_france.Anim_france_C|SetcanSlash _asanim_france false)
  (Game|SpawnActorfromClass "/Game/NewPlayers/Abiltys/player1Attack.player1Attack_C" (Transformation|GetWorldTransform (Variables|Default|GetArrow2)) "Undefined" 0 0)
  (bind _output_get (Variables|/Game/NewPlayers/BP_basePlayer.BP_basePlayer_C|SetWB_IngameHUD self (Variables|Default|GetWb_InGameHUD)))
  (Variables|/Game/NewPlayers/widgets/WB_InGameHUD.WB_InGameHUD_C|SetcanMonsterAttack _output_get false))

(event Custom|IfDead
  (if (<= (Variables|Default|GetHealth) 0.0)
    (Variables|Default|SetDead true)))

(event Custom|startSlash
  ;[1 1 1] slahs
  (bind _asanim_france (Utilities|Casting|CastToAnim_france (Components|SkeletalMesh|GetAnimInstance (Variables|Character|GetMesh))))
  (Variables|/Game/anim/Francesca/Animations/Anim_france.Anim_france_C|SetcanSlash _asanim_france false)
  (Game|SpawnActorfromClass "/Game/NewPlayers/Abiltys/player1Attack.player1Attack_C" (Transformation|GetWorldTransform (Variables|Default|GetArrow2)) "Undefined" 0 0)
  (bind _output_get (Variables|/Game/NewPlayers/BP_basePlayer.BP_basePlayer_C|SetWB_IngameHUD self (Variables|Default|GetWb_InGameHUD)))
  (Variables|/Game/NewPlayers/widgets/WB_InGameHUD.WB_InGameHUD_C|SetcanMonsterAttack _output_get false))

(event Custom|startCure
  ;[1 1 1] cure
  (AddComponent|AddAudioComponent false)
  (Game|SpawnActorfromClass "/Game/NewPlayers/Abiltys/cure.cure_C" (Transformation|GetWorldTransform (Variables|Default|GetArrow2)) "Undefined" 0 0)
  (Variables|Default|SetAntidote (- (Variables|Default|GetAntidote) 1)))

(event Custom|startCureMulti
  ;[1 1 1] cure
  (AddComponent|AddAudioComponent false)
  (Game|SpawnActorfromClass "/Game/NewPlayers/Abiltys/cure.cure_C" (Transformation|GetWorldTransform (Variables|Default|GetArrow2)) "Undefined" 0 0)
  (Variables|Default|SetAntidote (- (Variables|Default|GetAntidote) 1)))

(event Custom|startCureSever
  ;[1 1 1] cure
  (AddComponent|AddAudioComponent false)
  (Game|SpawnActorfromClass "/Game/NewPlayers/Abiltys/cure.cure_C" (Transformation|GetWorldTransform (Variables|Default|GetArrow2)) "Undefined" 0 0)
  (Variables|Default|SetAntidote (- (Variables|Default|GetAntidote) 1)))

(event Custom|startCrouchSever
  ;[1 1 1] crouch
  (bind _asanim_france (Utilities|Casting|CastToAnim_france (Components|SkeletalMesh|GetAnimInstance (Variables|Character|GetMesh))))
  (Variables|/Game/anim/Francesca/Animations/Anim_france.Anim_france_C|SetisCrouching _asanim_france true))

(event Custom|stopSlash
  ;[1 1 1] slahs
  (Utilities|FlowControl|Delay 1.47)
  (bind _asanim_france (Utilities|Casting|CastToAnim_france (Components|SkeletalMesh|GetAnimInstance (Variables|Character|GetMesh))))
  (Variables|/Game/anim/Francesca/Animations/Anim_france.Anim_france_C|SetcanSlash _asanim_france false))

(event Custom|startSetTrapSever
  ;[1 1 1] settrap
  (bind _asanim_france (Utilities|Casting|CastToAnim_france (Components|SkeletalMesh|GetAnimInstance (Variables|Character|GetMesh))))
  (Variables|/Game/anim/Francesca/Animations/Anim_france.Anim_france_C|SetcanSetTrap _asanim_france true)
  (Utilities|FlowControl|Delay 1.17)
  (Game|SpawnActorfromClass "/Game/NewPlayers/Abiltys/tripWire.tripWire_C" (Transformation|GetWorldTransform (Variables|Default|GetTripwireArrow)) "Undefined" 0 0)
  (bind _output_get (Variables|Default|SetTrip%20Wire (- (Variables|Default|GetTrip%20Wire) 1)))
  (if (<= _output_get 0)
    (bind _output_get_2 (Variables|/Game/NewPlayers/BP_basePlayer.BP_basePlayer_C|SetWB_IngameHUD self (Variables|Default|GetWb_InGameHUD)))
    (Variables|/Game/NewPlayers/widgets/WB_InGameHUD.WB_InGameHUD_C|SetcanSetTrap _output_get_2 false)))

(event Custom|stopCrouch
  ;[1 1 1] crouch
  (bind _asanim_france (Utilities|Casting|CastToAnim_france (Components|SkeletalMesh|GetAnimInstance (Variables|Character|GetMesh))))
  (Variables|/Game/anim/Francesca/Animations/Anim_france.Anim_france_C|SetisCrouching _asanim_france false))

(event EventBeginPlay)

(event Collision|EventActorBeginOverlap
  (params (OtherActor :type Actor%20Object%20Reference)))

(event EventTick
  (params (DeltaSeconds :type Float%20%28single-precision%29))
  (if (Variables|Default|GetIs%20Infected)
    (AI|Navigation|StopMovement (Game|GetPlayerController 0))
    (Development|SetHiddeninGame (Variables|Default|GetTextRender) false false)
    (Utilities|FlowControl|Delay 3e+01)
    (bind _output_get (Variables|/Game/NewPlayers/BP_basePlayer.BP_basePlayer_C|SetWB_IngameHUD self (Variables|Default|GetWb_InGameHUD)))
    (Variables|/Game/NewPlayers/widgets/WB_InGameHUD.WB_InGameHUD_C|Setturned _output_get true)
    (Input|EnableInput (Game|GetPlayerController 0))))

(fn ConstructionScript
  (Variables|Default|SetcharRowName "Player2")
  (|CallParentFunction))