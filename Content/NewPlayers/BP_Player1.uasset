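; Player 1 character with powder-ball throw, slash, cure and crouch actions plus infection and death states.
; Actions set Jimmy_Anim flags or spawn actors, updating ammo and HUD; local, multi and server events share each body.
; Tick checks Health and infection, which halts movement and marks the HUD turned after a delay.
; InfactArea overlap flags an antidote-carrying BP_Player2 to cure; construction sets the parent's character row name.
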(event OnComponentBeginOverlap(infactArea)
  (params (OverlappedComponent :type Primitive%20Component%20Object%20Reference) (OtherActor :type Actor%20Object%20Reference) (OtherComp :type Primitive%20Component%20Object%20Reference) (OtherBodyIndex :type Integer) (bFromSweep :type Boolean) (SweepResult :type Hit%20Result%20Structure%20%28by%20ref%29))
  ;[1 1 1] cure
  (bind _asbp_player_2 (Utilities|Casting|CastToBP_Player2 OtherActor))
  (if (> (Variables|/Game/NewPlayers/BP_basePlayer.BP_basePlayer_C|GetAntidote _asbp_player_2) 0)
    (Variables|/Game/NewPlayers/BP_basePlayer.BP_basePlayer_C|SetCure _asbp_player_2 true)
    (else
      (Development|PrintString "fealed" true true "(R=1.000000,G=0.000000,B=0.533423,A=1.000000)"))))

(event Custom|startCrouch
  ;[1 1 1] crouch
  (bind _asjimmy_anim (Utilities|Casting|CastToJimmy_Anim (Components|SkeletalMesh|GetAnimInstance (Variables|Character|GetMesh))))
  (Variables|/Game/anim/Jimmy/Animations/Jimmy_Anim.Jimmy_Anim_C|SetisCrouching _asjimmy_anim true))

(event Custom|startCrouchMulti
  ;[1 1 1] crouch
  (bind _asjimmy_anim (Utilities|Casting|CastToJimmy_Anim (Components|SkeletalMesh|GetAnimInstance (Variables|Character|GetMesh))))
  (Variables|/Game/anim/Jimmy/Animations/Jimmy_Anim.Jimmy_Anim_C|SetisCrouching _asjimmy_anim true))

(event Custom|stopCrouchMulti
  ;[1 1 1] crouch
  (bind _asjimmy_anim (Utilities|Casting|CastToJimmy_Anim (Components|SkeletalMesh|GetAnimInstance (Variables|Character|GetMesh))))
  (Variables|/Game/anim/Jimmy/Animations/Jimmy_Anim.Jimmy_Anim_C|SetisCrouching _asjimmy_anim false))

(event Custom|stopCrouchSever
  ;[1 1 1] crouch
  (bind _asjimmy_anim (Utilities|Casting|CastToJimmy_Anim (Components|SkeletalMesh|GetAnimInstance (Variables|Character|GetMesh))))
  (Variables|/Game/anim/Jimmy/Animations/Jimmy_Anim.Jimmy_Anim_C|SetisCrouching _asjimmy_anim false))

(event Custom|startThrowPowderBall
  ;[1 1 1] ThrowPowderBall
  (bind _asjimmy_anim (Utilities|Casting|CastToJimmy_Anim (Components|SkeletalMesh|GetAnimInstance (Variables|Character|GetMesh))))
  (Variables|/Game/anim/Jimmy/Animations/Jimmy_Anim.Jimmy_Anim_C|SetcanThrow _asjimmy_anim true)
  (Utilities|FlowControl|Delay 0.39)
  (Game|SpawnActorfromClass "/Game/NewPlayers/Abiltys/powderBall.powderBall_C" (Transformation|GetWorldTransform (Variables|Default|GetpowderBallArrow)) "Undefined" 0 0)
  (bind _output_get (Variables|Default|SetPowder%20Ball (- (Variables|Default|GetPowder%20Ball) 1)))
  (if (<= _output_get 0)
    (bind _output_get_2 (Variables|/Game/NewPlayers/BP_basePlayer.BP_basePlayer_C|SetWB_IngameHUD self (Variables|Default|GetWb_InGameHUD)))
    (Variables|/Game/NewPlayers/widgets/WB_InGameHUD.WB_InGameHUD_C|SetcanThrowPowderBall _output_get_2 false)))

(event Custom|startThrowPowderBallMulti
  ;[1 1 1] ThrowPowderBall
  (bind _asjimmy_anim (Utilities|Casting|CastToJimmy_Anim (Components|SkeletalMesh|GetAnimInstance (Variables|Character|GetMesh))))
  (Variables|/Game/anim/Jimmy/Animations/Jimmy_Anim.Jimmy_Anim_C|SetcanThrow _asjimmy_anim true)
  (Utilities|FlowControl|Delay 0.39)
  (Game|SpawnActorfromClass "/Game/NewPlayers/Abiltys/powderBall.powderBall_C" (Transformation|GetWorldTransform (Variables|Default|GetpowderBallArrow)) "Undefined" 0 0)
  (bind _output_get (Variables|Default|SetPowder%20Ball (- (Variables|Default|GetPowder%20Ball) 1)))
  (if (<= _output_get 0)
    (bind _output_get_2 (Variables|/Game/NewPlayers/BP_basePlayer.BP_basePlayer_C|SetWB_IngameHUD self (Variables|Default|GetWb_InGameHUD)))
    (Variables|/Game/NewPlayers/widgets/WB_InGameHUD.WB_InGameHUD_C|SetcanThrowPowderBall _output_get_2 false)))

(event Custom|startSlashMulti
  ;[1 1 1] whenInfected
  (bind _asjimmy_anim (Utilities|Casting|CastToJimmy_Anim (Components|SkeletalMesh|GetAnimInstance (Variables|Character|GetMesh))))
  (Variables|/Game/anim/Jimmy/Animations/Jimmy_Anim.Jimmy_Anim_C|SetcanSlash _asjimmy_anim true)
  (Game|SpawnActorfromClass "/Game/NewPlayers/Abiltys/player1Attack.player1Attack_C" (Transformation|GetWorldTransform (Variables|Default|GetArrow2)) "Undefined" 0 0)
  (bind _output_get (Variables|/Game/NewPlayers/BP_basePlayer.BP_basePlayer_C|SetWB_IngameHUD self (Variables|Default|GetWb_InGameHUD)))
  (Variables|/Game/NewPlayers/widgets/WB_InGameHUD.WB_InGameHUD_C|SetcanMonsterAttack _output_get false))

(event Custom|startThrowPowderBallSever
  ;[1 1 1] ThrowPowderBall
  (bind _asjimmy_anim (Utilities|Casting|CastToJimmy_Anim (Components|SkeletalMesh|GetAnimInstance (Variables|Character|GetMesh))))
  (Variables|/Game/anim/Jimmy/Animations/Jimmy_Anim.Jimmy_Anim_C|SetcanThrow _asjimmy_anim true)
  (Utilities|FlowControl|Delay 0.39)
  (Game|SpawnActorfromClass "/Game/NewPlayers/Abiltys/powderBall.powderBall_C" (Transformation|GetWorldTransform (Variables|Default|GetpowderBallArrow)) "Undefined" 0 0)
  (bind _output_get (Variables|Default|SetPowder%20Ball (- (Variables|Default|GetPowder%20Ball) 1)))
  (if (<= _output_get 0)
    (bind _output_get_2 (Variables|/Game/NewPlayers/BP_basePlayer.BP_basePlayer_C|SetWB_IngameHUD self (Variables|Default|GetWb_InGameHUD)))
    (Variables|/Game/NewPlayers/widgets/WB_InGameHUD.WB_InGameHUD_C|SetcanThrowPowderBall _output_get_2 false)))

(event Custom|stopThrowPowderBall
  ;[1 1 1] ThrowPowderBall
  (Utilities|FlowControl|Delay 1.76)
  (bind _asjimmy_anim (Utilities|Casting|CastToJimmy_Anim (Components|SkeletalMesh|GetAnimInstance (Variables|Character|GetMesh))))
  (Variables|/Game/anim/Jimmy/Animations/Jimmy_Anim.Jimmy_Anim_C|SetcanThrow _asjimmy_anim false))

(event Custom|stopSlash
  ;[1 1 1] whenInfected
  (Utilities|FlowControl|Delay 1.47)
  (bind _asjimmy_anim (Utilities|Casting|CastToJimmy_Anim (Components|SkeletalMesh|GetAnimInstance (Variables|Character|GetMesh))))
  (Variables|/Game/anim/Jimmy/Animations/Jimmy_Anim.Jimmy_Anim_C|SetcanSlash _asjimmy_anim false))

(event Custom|stopSlashMulti
  ;[1 1 1] whenInfected
  (Utilities|FlowControl|Delay 1.47)
  (bind _asjimmy_anim (Utilities|Casting|CastToJimmy_Anim (Components|SkeletalMesh|GetAnimInstance (Variables|Character|GetMesh))))
  (Variables|/Game/anim/Jimmy/Animations/Jimmy_Anim.Jimmy_Anim_C|SetcanSlash _asjimmy_anim false))

(event Custom|stopSlashSever
  ;[1 1 1] whenInfected
  (Utilities|FlowControl|Delay 1.47)
  (bind _asjimmy_anim (Utilities|Casting|CastToJimmy_Anim (Components|SkeletalMesh|GetAnimInstance (Variables|Character|GetMesh))))
  (Variables|/Game/anim/Jimmy/Animations/Jimmy_Anim.Jimmy_Anim_C|SetcanSlash _asjimmy_anim false))

(event Custom|startSlashServer
  ;[1 1 1] whenInfected
  (bind _asjimmy_anim (Utilities|Casting|CastToJimmy_Anim (Components|SkeletalMesh|GetAnimInstance (Variables|Character|GetMesh))))
  (Variables|/Game/anim/Jimmy/Animations/Jimmy_Anim.Jimmy_Anim_C|SetcanSlash _asjimmy_anim true)
  (Game|SpawnActorfromClass "/Game/NewPlayers/Abiltys/player1Attack.player1Attack_C" (Transformation|GetWorldTransform (Variables|Default|GetArrow2)) "Undefined" 0 0)
  (bind _output_get (Variables|/Game/NewPlayers/BP_basePlayer.BP_basePlayer_C|SetWB_IngameHUD self (Variables|Default|GetWb_InGameHUD)))
  (Variables|/Game/NewPlayers/widgets/WB_InGameHUD.WB_InGameHUD_C|SetcanMonsterAttack _output_get false))

(event Custom|stopThrowPowderBallMulti
  ;[1 1 1] ThrowPowderBall
  (Utilities|FlowControl|Delay 1.76)
  (bind _asjimmy_anim (Utilities|Casting|CastToJimmy_Anim (Components|SkeletalMesh|GetAnimInstance (Variables|Character|GetMesh))))
  (Variables|/Game/anim/Jimmy/Animations/Jimmy_Anim.Jimmy_Anim_C|SetcanThrow _asjimmy_anim false))

(event Custom|stopThrowPowderBallSever
  ;[1 1 1] ThrowPowderBall
  (Utilities|FlowControl|Delay 1.76)
  (bind _asjimmy_anim (Utilities|Casting|CastToJimmy_Anim (Components|SkeletalMesh|GetAnimInstance (Variables|Character|GetMesh))))
  (Variables|/Game/anim/Jimmy/Animations/Jimmy_Anim.Jimmy_Anim_C|SetcanThrow _asjimmy_anim false))

(event Custom|startSlash
  ;[1 1 1] whenInfected
  (bind _asjimmy_anim (Utilities|Casting|CastToJimmy_Anim (Components|SkeletalMesh|GetAnimInstance (Variables|Character|GetMesh))))
  (Variables|/Game/anim/Jimmy/Animations/Jimmy_Anim.Jimmy_Anim_C|SetcanSlash _asjimmy_anim true)
  (Game|SpawnActorfromClass "/Game/NewPlayers/Abiltys/player1Attack.player1Attack_C" (Transformation|GetWorldTransform (Variables|Default|GetArrow2)) "Undefined" 0 0)
  (bind _output_get (Variables|/Game/NewPlayers/BP_basePlayer.BP_basePlayer_C|SetWB_IngameHUD self (Variables|Default|GetWb_InGameHUD)))
  (Variables|/Game/NewPlayers/widgets/WB_InGameHUD.WB_InGameHUD_C|SetcanMonsterAttack _output_get false))

(event Custom|startCure
  ;[1 1 1] cure
  (AddComponent|AddAudioComponent false)
  (Game|SpawnActorfromClass "/Game/NewPlayers/Abiltys/cure.cure_C" (Transformation|GetWorldTransform (Variables|Default|GetArrow2)) "Undefined" 0 0)
  (Variables|Default|SetAntidote (- (Variables|Default|GetAntidote) 1)))

(event Custom|startCureMulti
  ;[1 1 1] cure
  (AddComponent|AddAudioComponent false)
  (Game|SpawnActorfromClass "/Game/NewPlayers/Abiltys/cure.cure_C" (Transformation|GetWorldTransform (Variables|Default|GetArrow2)) "Undefined" 0 0)
  (Variables|Default|SetAntidote (- (Variables|Default|GetAntidote) 1)))

(event Custom|startCureSever
  ;[1 1 1] cure
  (AddComponent|AddAudioComponent false)
  (Game|SpawnActorfromClass "/Game/NewPlayers/Abiltys/cure.cure_C" (Transformation|GetWorldTransform (Variables|Default|GetArrow2)) "Undefined" 0 0)
  (Variables|Default|SetAntidote (- (Variables|Default|GetAntidote) 1)))

(event Custom|startCrouchSever
  ;[1 1 1] crouch
  (bind _asjimmy_anim (Utilities|Casting|CastToJimmy_Anim (Components|SkeletalMesh|GetAnimInstance (Variables|Character|GetMesh))))
  (Variables|/Game/anim/Jimmy/Animations/Jimmy_Anim.Jimmy_Anim_C|SetisCrouching _asjimmy_anim true))

(event Custom|IfDead
  (if (<= (Variables|Default|GetHealth) 0.0)
    (Variables|Default|SetDead true)))

(event Custom|gettingInfacted
  ;[1 1 1] getsInfected
  (if (Variables|Default|GetIs%20Infected)
    (Components|Movement|StopMovementImmediately (Variables|Character|GetCharacterMovement))
    (Development|SetHiddeninGame (Variables|Default|GetTextRender) false false)
    (Utilities|FlowControl|Delay 3e+01)
    (if (Variables|Default|GetIs%20Infected)
      (Input|EnableInput self (Game|GetPlayerController 0))
      (bind _output_get (Variables|/Game/NewPlayers/BP_basePlayer.BP_basePlayer_C|SetWB_IngameHUD self (Variables|Default|GetWb_InGameHUD)))
      (Variables|/Game/NewPlayers/widgets/WB_InGameHUD.WB_InGameHUD_C|Setturned _output_get true))
    (else
      (Input|EnableInput self (Game|GetPlayerController 0))
      (Development|SetHiddeninGame (Variables|Default|GetTextRender) true false))))

(event Custom|stopCrouch
  ;[1 1 1] crouch
  (bind _asjimmy_anim (Utilities|Casting|CastToJimmy_Anim (Components|SkeletalMesh|GetAnimInstance (Variables|Character|GetMesh))))
  (Variables|/Game/anim/Jimmy/Animations/Jimmy_Anim.Jimmy_Anim_C|SetisCrouching _asjimmy_anim false))

(event EventTick
  (params (DeltaSeconds :type Float%20%28single-precision%29))
  (Utilities|FlowControl|Sequence
    (:then_0
      (CallFunction|GettingInfacted))
    (:then_1
      (CallFunction|IfDead))))

(fn ConstructionScript
  (Variables|Default|SetcharRowName "Player1")
  (|CallParentFunction))