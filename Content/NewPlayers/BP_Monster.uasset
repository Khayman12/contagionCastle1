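; Playable Monster character, a child class using the "Monster" row name, with slash, trap and infect abilities.
; Abilities spawn actors at arrow components through events with Server and Multi variants; slash also drives the anim blueprint, and slash and trap clear HUD availability flags.
; InfactArea overlaps toggle a HUD infect flag based on player health and infection.
; Trip and stun disable input temporarily; ragdoll toggling is unwired, though capsule-tracking logic remains.
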(event OnComponentBeginOverlap(infactArea)
  (params (OverlappedComponent :type Primitive%20Component%20Object%20Reference) (OtherActor :type Actor%20Object%20Reference) (OtherComp :type Primitive%20Component%20Object%20Reference) (OtherBodyIndex :type Integer) (bFromSweep :type Boolean) (SweepResult :type Hit%20Result%20Structure%20%28by%20ref%29))
  ;[1 1 1] InfactPlayers
  (CallFunction|CheackPlayersHealth OtherActor))

(event OnComponentEndOverlap(infactArea)
  (params (OverlappedComponent :type Primitive%20Component%20Object%20Reference) (OtherActor :type Actor%20Object%20Reference) (OtherComp :type Primitive%20Component%20Object%20Reference) (OtherBodyIndex :type Integer))
  ;[1 1 1] InfactPlayers
  (bind _output_get (Variables|/Game/NewPlayers/BP_basePlayer.BP_basePlayer_C|SetWB_IngameHUD self (Variables|Default|GetWb_InGameHUD)))
  (Variables|/Game/NewPlayers/widgets/WB_InGameHUD.WB_InGameHUD_C|SetcanNotInfect _output_get false))

(event Custom|cheackPlayersHealth
  (params (Object :type Object%20Object%20Reference))
  ;[1 1 1] InfactPlayers
  (Utilities|FlowControl|Sequence
    (:then_0
      (bind _asbp_player_1 (Utilities|Casting|CastToBP_Player1 Object))
      (if (not (Variables|/Game/NewPlayers/BP_basePlayer.BP_basePlayer_C|GetIs%20Infected _asbp_player_1))
        (if (<= (Variables|/Game/NewPlayers/BP_basePlayer.BP_basePlayer_C|GetHealth _asbp_player_1) 5.0)
          (bind _output_get (Variables|/Game/NewPlayers/BP_basePlayer.BP_basePlayer_C|SetWB_IngameHUD self (Variables|Default|GetWb_InGameHUD)))
          (Variables|/Game/NewPlayers/widgets/WB_InGameHUD.WB_InGameHUD_C|SetcanNotInfect _output_get true))))
    (:then_1
      (bind _asbp_player_2 (Utilities|Casting|CastToBP_Player2 Object))
      (if (not (Variables|/Game/NewPlayers/BP_basePlayer.BP_basePlayer_C|GetIs%20Infected _asbp_player_2))
        (if (<= (Variables|/Game/NewPlayers/BP_basePlayer.BP_basePlayer_C|GetHealth _asbp_player_2) 5.0)
          (bind _output_get_2 (Variables|/Game/NewPlayers/BP_basePlayer.BP_basePlayer_C|SetWB_IngameHUD self (Variables|Default|GetWb_InGameHUD)))
          (Variables|/Game/NewPlayers/widgets/WB_InGameHUD.WB_InGameHUD_C|SetcanNotInfect _output_get_2 true))))))

(event Custom|startSetMonsterTrap
  ;[1 1 1] setTrap
  (Game|SpawnActorfromClass "/Game/NewPlayers/MonsterAbiltys/Pingbox.Pingbox_C" (Transformation|GetWorldTransform (Variables|Default|GetsetTrapArrow)) "Undefined" 0 0)
  (bind _output_get (Variables|/Game/NewPlayers/BP_basePlayer.BP_basePlayer_C|SetWB_IngameHUD self (Variables|Default|GetWb_InGameHUD)))
  (Variables|/Game/NewPlayers/widgets/WB_InGameHUD.WB_InGameHUD_C|SetcanMonsterSetTrap _output_get false))

(event Custom|TrackCapsul
  (bind _mesh (Variables|Character|GetMesh))
  (bind _returnvalue (Transformation|GetSocketLocation _mesh "Hips"))
  (if (Variables|Default|GetRagdolling)
    (bind (_outhit _returnvalue_2) (Collision|LineTraceByChannel _returnvalue (+ _returnvalue "0,0,-100.000000") "TraceTypeQuery1" false 0 "ForDuration"))
    (if _returnvalue_2
      (Variables|Default|SettargetGroundLocation (.Location (Collision|BreakHitResult _outhit)))
      (else
        (Variables|Default|SettargetGroundLocation (Transformation|GetSocketLocation (Variables|Character|GetMesh) "Hips"))))
    (bind _output_get (Variables|Default|SetmeshLocation (- (Variables|Default|GetHipOfSet) (Variables|Default|GettargetGroundLocation))))
    (Transformation|SetWorldLocation (Variables|Default|GetCapsuleComponent) _output_get false false)))

(event Custom|InitPhysicSetup
  (Variables|Default|SetHipOfSet (Variables|/Script/Engine.SceneComponent|GetRelativeLocation (Variables|Character|GetMesh))))

(event Custom|TrackCapMulti
  (bind _mesh (Variables|Character|GetMesh))
  (bind _returnvalue (Transformation|GetSocketLocation _mesh "Hips"))
  (if (Variables|Default|GetRagdolling)
    (bind (_outhit _returnvalue_2) (Collision|LineTraceByChannel _returnvalue (+ _returnvalue "0,0,-100.000000") "TraceTypeQuery1" false 0 "ForDuration"))
    (if _returnvalue_2
      (Variables|Default|SettargetGroundLocation (.Location (Collision|BreakHitResult _outhit)))
      (else
        (Variables|Default|SettargetGroundLocation (Transformation|GetSocketLocation (Variables|Character|GetMesh) "Hips"))))
    (bind _output_get (Variables|Default|SetmeshLocation (- (Variables|Default|GetHipOfSet) (Variables|Default|GettargetGroundLocation))))
    (Transformation|SetWorldLocation (Variables|Default|GetCapsuleComponent) _output_get false false)))

(event Custom|TrackCapSever
  (bind _mesh (Variables|Character|GetMesh))
  (bind _returnvalue (Transformation|GetSocketLocation _mesh "Hips"))
  (if (Variables|Default|GetRagdolling)
    (bind (_outhit _returnvalue_2) (Collision|LineTraceByChannel _returnvalue (+ _returnvalue "0,0,-100.000000") "TraceTypeQuery1" false 0 "ForDuration"))
    (if _returnvalue_2
      (Variables|Default|SettargetGroundLocation (.Location (Collision|BreakHitResult _outhit)))
      (else
        (Variables|Default|SettargetGroundLocation (Transformation|GetSocketLocation (Variables|Character|GetMesh) "Hips"))))
    (bind _output_get (Variables|Default|SetmeshLocation (- (Variables|Default|GetHipOfSet) (Variables|Default|GettargetGroundLocation))))
    (Transformation|SetWorldLocation (Variables|Default|GetCapsuleComponent) _output_get false false)))

(event Custom|startSlashMulti
  ;[1 1 1] start slash / stop Slash
  (bind _asnew_anim_blueprint (Utilities|Casting|CastToNewAnimBlueprint (Components|SkeletalMesh|GetAnimInstance (Variables|Character|GetMesh))))
  (Variables|/Game/anim/monster/NewAnimBlueprint.NewAnimBlueprint_C|SetisSlash _asnew_anim_blueprint true)
  (Game|SpawnActorfromClass "/Game/NewPlayers/MonsterAbiltys/MonsterAttack.MonsterAttack_C" (Transformation|GetWorldTransform (Variables|Default|GetArrow2)) "Undefined" 0 0)
  (bind _output_get (Variables|/Game/NewPlayers/BP_basePlayer.BP_basePlayer_C|SetWB_IngameHUD self (Variables|Default|GetWb_InGameHUD)))
  (Variables|/Game/NewPlayers/widgets/WB_InGameHUD.WB_InGameHUD_C|SetcanMonsterAttack _output_get false))

(event Custom|gotHitWithPowderBall
  ;[1 1 1] GotStunned
  (if (Variables|Default|Getstunned)
    (Input|DisableInput (Game|GetPlayerController 0))
    (Utilities|FlowControl|Delay 1e+01)
    (Variables|Default|Setstunned false)
    (else
      (Input|EnableInput (Game|GetPlayerController 0)))))

(event Custom|gotTrippedSever
  ;[1 1 1] got Tripped
  (if (Variables|Default|Gettripped)
    (Input|DisableInput (Game|GetPlayerController 0))
    (Utilities|FlowControl|Delay 1e+01)
    (Variables|Default|Settripped false)
    (else
      (Input|EnableInput (Game|GetPlayerController 0)))))

(event Custom|stopSlash
  ;[1 1 1] start slash / stop Slash
  (Utilities|FlowControl|Delay 1.5)
  (bind _asnew_anim_blueprint (Utilities|Casting|CastToNewAnimBlueprint (Components|SkeletalMesh|GetAnimInstance (Variables|Character|GetMesh))))
  (Variables|/Game/anim/monster/NewAnimBlueprint.NewAnimBlueprint_C|SetisSlash _asnew_anim_blueprint false))

(event Custom|stopSlashMulti
  ;[1 1 1] start slash / stop Slash
  (Utilities|FlowControl|Delay 1.5)
  (bind _asnew_anim_blueprint (Utilities|Casting|CastToNewAnimBlueprint (Components|SkeletalMesh|GetAnimInstance (Variables|Character|GetMesh))))
  (Variables|/Game/anim/monster/NewAnimBlueprint.NewAnimBlueprint_C|SetisSlash _asnew_anim_blueprint false))

(event Custom|stopSlashSever
  ;[1 1 1] start slash / stop Slash
  (Utilities|FlowControl|Delay 1.5)
  (bind _asnew_anim_blueprint (Utilities|Casting|CastToNewAnimBlueprint (Components|SkeletalMesh|GetAnimInstance (Variables|Character|GetMesh))))
  (Variables|/Game/anim/monster/NewAnimBlueprint.NewAnimBlueprint_C|SetisSlash _asnew_anim_blueprint false))

(event Custom|startSlashServer
  ;[1 1 1] start slash / stop Slash
  (bind _asnew_anim_blueprint (Utilities|Casting|CastToNewAnimBlueprint (Components|SkeletalMesh|GetAnimInstance (Variables|Character|GetMesh))))
  (Variables|/Game/anim/monster/NewAnimBlueprint.NewAnimBlueprint_C|SetisSlash _asnew_anim_blueprint true)
  (Game|SpawnActorfromClass "/Game/NewPlayers/MonsterAbiltys/MonsterAttack.MonsterAttack_C" (Transformation|GetWorldTransform (Variables|Default|GetArrow2)) "Undefined" 0 0)
  (bind _output_get (Variables|/Game/NewPlayers/BP_basePlayer.BP_basePlayer_C|SetWB_IngameHUD self (Variables|Default|GetWb_InGameHUD)))
  (Variables|/Game/NewPlayers/widgets/WB_InGameHUD.WB_InGameHUD_C|SetcanMonsterAttack _output_get false))

(event Custom|StopInfectPlayers
  ;[1 1 1] InfactPlayers
)

(event Custom|StopInfactPlayersMulti
  ;[1 1 1] InfactPlayers
)

(event Custom|StopInfactPlayersSever
  ;[1 1 1] InfactPlayers
)

(event Custom|StartInfectPlayers
  ;[1 1 1] InfactPlayers
  (Game|SpawnActorfromClass "/Game/NewPlayers/MonsterAbiltys/infactePlayer.infactePlayer_C" (Transformation|GetWorldTransform (Variables|Default|GetArrow2)) "Undefined" 0 0))

(event Custom|StartInfactPlayersMulti
  ;[1 1 1] InfactPlayers
  (Game|SpawnActorfromClass "/Game/NewPlayers/MonsterAbiltys/infactePlayer.infactePlayer_C" (Transformation|GetWorldTransform (Variables|Default|GetArrow2)) "Undefined" 0 0))

(event Custom|StartInfactPlayersSever
  ;[1 1 1] InfactPlayers
  (Game|SpawnActorfromClass "/Game/NewPlayers/MonsterAbiltys/infactePlayer.infactePlayer_C" (Transformation|GetWorldTransform (Variables|Default|GetArrow2)) "Undefined" 0 0))

(event Custom|startSlash
  ;[1 1 1] start slash / stop Slash
  (bind _asnew_anim_blueprint (Utilities|Casting|CastToNewAnimBlueprint (Components|SkeletalMesh|GetAnimInstance (Variables|Character|GetMesh))))
  (Variables|/Game/anim/monster/NewAnimBlueprint.NewAnimBlueprint_C|SetisSlash _asnew_anim_blueprint true)
  (Game|SpawnActorfromClass "/Game/NewPlayers/MonsterAbiltys/MonsterAttack.MonsterAttack_C" (Transformation|GetWorldTransform (Variables|Default|GetArrow2)) "Undefined" 0 0)
  (bind _output_get (Variables|/Game/NewPlayers/BP_basePlayer.BP_basePlayer_C|SetWB_IngameHUD self (Variables|Default|GetWb_InGameHUD)))
  (Variables|/Game/NewPlayers/widgets/WB_InGameHUD.WB_InGameHUD_C|SetcanMonsterAttack _output_get false))

(event Custom|stopSetMomsterTrap
  ;[1 1 1] setTrap
)

(event Custom|stopSetMonsterTrapMulti
  ;[1 1 1] setTrap
)

(event Custom|stopSetMonsterTrapSever
  ;[1 1 1] setTrap
)

(event Custom|gotTripped
  ;[1 1 1] got Tripped
  (if (Variables|Default|Gettripped)
    (Input|DisableInput (Game|GetPlayerController 0))
    (Utilities|FlowControl|Delay 1e+01)
    (Variables|Default|Settripped false)
    (else
      (Input|EnableInput (Game|GetPlayerController 0)))))

(event Custom|startSetMonsterTrapMulti
  ;[1 1 1] setTrap
  (Game|SpawnActorfromClass "/Game/NewPlayers/MonsterAbiltys/Pingbox.Pingbox_C" (Transformation|GetWorldTransform (Variables|Default|GetsetTrapArrow)) "Undefined" 0 0)
  (bind _output_get (Variables|/Game/NewPlayers/BP_basePlayer.BP_basePlayer_C|SetWB_IngameHUD self (Variables|Default|GetWb_InGameHUD)))
  (Variables|/Game/NewPlayers/widgets/WB_InGameHUD.WB_InGameHUD_C|SetcanMonsterSetTrap _output_get false))

(event Custom|startSetMonsterTrapSever
  ;[1 1 1] setTrap
  (Game|SpawnActorfromClass "/Game/NewPlayers/MonsterAbiltys/Pingbox.Pingbox_C" (Transformation|GetWorldTransform (Variables|Default|GetsetTrapArrow)) "Undefined" 0 0)
  (bind _output_get (Variables|/Game/NewPlayers/BP_basePlayer.BP_basePlayer_C|SetWB_IngameHUD self (Variables|Default|GetWb_InGameHUD)))
  (Variables|/Game/NewPlayers/widgets/WB_InGameHUD.WB_InGameHUD_C|SetcanMonsterSetTrap _output_get false))

(event Custom|gotTrippedMulti
  ;[1 1 1] got Tripped
  (if (Variables|Default|Gettripped)
    (Input|DisableInput (Game|GetPlayerController 0))
    (Utilities|FlowControl|Delay 1e+01)
    (Variables|Default|Settripped false)
    (else
      (Input|EnableInput (Game|GetPlayerController 0)))))

(event EventBeginPlay)

(event EventTick
  (params (DeltaSeconds :type Float%20%28single-precision%29)))

(fn ConstructionScript
  (Variables|Default|SetcharRowName "Monster")
  (|CallParentFunction))