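; In-game PlayerController that sets up a local player's HUD, game-only input and saved profile.
; On BeginPlay it creates the HUD widget and loads the profile from a save slot, passing it through a server event when not authority.
; On possession it waits briefly, then hands the HUD to the BP_basePlayer pawn and refreshes health.
; Further events re-enable pawn input and trigger the HUD's game-start countdown.
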(event Custom|Local_SetHUDVar
  (bind _wb_ingamehud (Variables|Default|GetWb_InGameHUD))
  (Utilities|FlowControl|Delay 0.2)
  (bind _asbp_base_player (Utilities|Casting|CastToBP_basePlayer (Pawn|GetControlledPawn)))
  (Variables|/Game/NewPlayers/BP_basePlayer.BP_basePlayer_C|SetWB_IngameHUD _asbp_base_player _wb_ingamehud)
  (Default|UpdateHealth _wb_ingamehud (Variables|/Game/NewPlayers/BP_basePlayer.BP_basePlayer_C|GetHealth _asbp_base_player)))

(event Custom|Svr_SetplayerProfile
  (params (S_playerProfile :type S%20Player%20Profile%20Structure))
  (Variables|Default|SetS_playerProfile S_playerProfile))

(event Custom|EnableAlInput
  (Input|EnableInput (Pawn|GetControlledPawn) self))

(event Custom|GamestartCountDown
  (Default|GameStartCountDown (Variables|Default|GetWb_InGameHUD)))

(event EventBeginPlay
  (if (Pawn|IsLocalPlayerController)
    (Viewport|RemoveAllWidgets)
    (CallFunction|UIShowinGameHUD)
    (Input|SetInputModeGameOnly self)
    (Variables|Default|SetbShowMouseCursor false)
    (bind _returnvalue (SaveGame|LoadGamefromSlot "PlayerProfile_Slot"))
    (bind _assg_player_profile (Utilities|Casting|CastToSG_PlayerProfile _returnvalue))
    (Networking|SwitchHasAuthority
      (:Authority
        (Variables|Default|SetS_playerProfile (Variables|/Game/SaveData/SG_PlayerProfile.SG_PlayerProfile_C|GetplayerProfile _assg_player_profile)))
      (:Remote
        (CallFunction|SvrSetplayerProfile (Variables|/Game/SaveData/SG_PlayerProfile.SG_PlayerProfile_C|GetplayerProfile _assg_player_profile))))))

(event EventTick
  (params (DeltaSeconds :type Float%20%28single-precision%29)))

(event EventPossess
  (params (PossessedPawn :type Pawn%20Object%20Reference))
  (CallFunction|LocalSetHUDVar))

(fn ConstructionScript)

(fn UIShowinGameHUD
  (Utilities|IsValid (Variables|Default|GetWb_InGameHUD)
    (:Is%20Valid
      _)
    (:Is%20Not%20Valid
      (bind _returnvalue (UserInterface|CreateWidget "/Game/NewPlayers/widgets/WB_InGameHUD.WB_InGameHUD_C" self))
      (bind _output_get (Variables|Default|SetWb_InGameHUD _returnvalue))))
  (UserInterface|Viewport|AddtoViewport _output_get 0)
  (return))