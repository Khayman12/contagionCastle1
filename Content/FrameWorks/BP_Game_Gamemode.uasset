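; Game mode for multiplayer matches that waits for every expected player, spawns their chosen characters and starts the level together.
; New controllers are tracked until their count matches the GameInstance's connected-player count, then each restarts at a player start named by its index.
; Pawn spawning takes the character class from PlayerState or PlayerController depending on seamless travel, and updates a minimap widget.
; LevelStart then runs a countdown on all controllers and enables their input.
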(event Custom|LevelStart
  (Utilities|FlowControl|Delay 0.2)
  (for _array_element (Variables|Default|GetAll_ConnectedControllers)
    (Default|GamestartCountDown _array_element))
  (Utilities|FlowControl|Delay 3.0)
  (for _array_element_2 (Variables|Default|GetAll_ConnectedControllers)
    (Default|EnableAlInput _array_element_2)))

(event EventBeginPlay
  (bind _asbp_game_game_instance (Utilities|Casting|CastToBP_Game_GameInstance (Game|GetGameInstance)))
  (Variables|Default|SetbUseSeamlessTravel (Variables|/Game/FrameWorks/BP_Game_GameInstance.BP_Game_GameInstance_C|GetSeamlessTravelEnabled _asbp_game_game_instance))
  (Variables|Default|SetSeamless%20Travel%20Enabled (Variables|/Game/FrameWorks/BP_Game_GameInstance.BP_Game_GameInstance_C|GetSeamlessTravelEnabled _asbp_game_game_instance)))

(event EventHandleStartingNewPlayer
  (params (NewPlayer :type Player%20Controller%20Object%20Reference))
  (bind _asbp_game_player_controller (Utilities|Casting|CastToBP_Game_PlayerController NewPlayer))
  (Utilities|Array|Add (Variables|Default|GetAll_ConnectedControllers) _asbp_game_player_controller)
  (bind _asbp_game_game_instance (Utilities|Casting|CastToBP_Game_GameInstance (Game|GetGameInstance)))
  (Variables|Default|SetNum_ExpectedPlayers (Variables|/Game/FrameWorks/BP_Game_GameInstance.BP_Game_GameInstance_C|GetNum%20Connected%20Players _asbp_game_game_instance))
  (if (== (Variables|Default|GetNum_ExpectedPlayers) (Utilities|Array|Length (Variables|Default|GetAll_ConnectedControllers)))
    (Utilities|FlowControl|Delay 0.5)
    (for (_array_element _array_index) (Variables|Default|GetAll_ConnectedControllers)
      (Development|PrintString "Restart" true true "(R=1.000000,G=0.000000,B=0.812734,A=1.000000)" 3e+01)
      (Class|GameModeBase|RestartPlayeratPlayerStart _array_element (Class|GameModeBase|FindPlayerStart _array_element (Utilities|String|ToString(Integer) _array_index))))
    (CallFunction|LevelStart)
    (else
      (Development|PrintString "feiled to get all players" true true "(R=0.000000,G=1.000000,B=0.216045,A=1.000000)" 1e+01))))

(event EventOnLogout
  (params (ExitingController :type Controller%20Object%20Reference))
  (bind _asbp_game_player_controller (Utilities|Casting|CastToBP_Game_PlayerController ExitingController))
  (Utilities|Array|RemoveItem (Variables|Default|GetAll_ConnectedControllers) _asbp_game_player_controller)
  (Math|Integer|DecrementInt (Variables|Default|GetNum_ExpectedPlayers)))

(fn ConstructionScript)

(fn SpawnDefaultPawnfor
  (params (NewPlayer :type Controller%20Object%20Reference) (StartSpot :type Actor%20Object%20Reference))
  (if (Variables|Default|GetSeamless%20Travel%20Enabled)
    (bind _asbp_game_player_state (Utilities|Casting|CastToBP_Game_PlayerState (Variables|/Script/Engine.Controller|GetPlayerState NewPlayer)))
    (LocalVariables|SetLcl_CharacterClass (.characterclass (Variables|/Game/FrameWorks/BP_Game_PlayerState.BP_Game_PlayerState_C|GetS_PlayerProfile _asbp_game_player_state)))
    (bind _returnvalue (UserInterface|CreateWidget "/Game/MiniMap/WightStuff/WB_MiniMap.WB_MiniMap_C"))
    (Default|UpdateMap2 _returnvalue (.charrowname (Variables|/Game/FrameWorks/BP_Game_PlayerState.BP_Game_PlayerState_C|GetS_PlayerProfile _asbp_game_player_state)))
    (else
      (bind _asbp_game_player_controller (Utilities|Casting|CastToBP_Game_PlayerController NewPlayer))
      (LocalVariables|SetLcl_CharacterClass (.characterclass (Variables|/Game/FrameWorks/BP_Game_PlayerController.BP_Game_PlayerController_C|GetS_playerProfile _asbp_game_player_controller)))
      (bind _returnvalue_2 (UserInterface|CreateWidget "/Game/MiniMap/WightStuff/WB_MiniMap.WB_MiniMap_C"))
      (Default|UpdateMap2 _returnvalue_2 (.charrowname (Variables|/Game/FrameWorks/BP_Game_PlayerController.BP_Game_PlayerController_C|GetS_playerProfile _asbp_game_player_controller)))))
  (bind _returnvalue_3 (Game|SpawnActorfromClass (LocalVariables|GetLcl_CharacterClass) (Transformation|GetActorTransform StartSpot) "Undefined" 0 0))
  (bind _asbp_base_player (Utilities|Casting|CastToBP_basePlayer _returnvalue_3))
  (return _asbp_base_player))