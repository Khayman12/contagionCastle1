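; Game instance that manages the player profile, the main menu and server map travel.
; Showing the main menu creates the widget, switches to UI-only input, then loads the saved profile to fill the name field.
; Name changes write the profile to a SaveGame slot, though a missing save object is only created, not written.
; TravelToMap runs a servertravel console command; the multiplayer menu function is an empty stub.
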(event Custom|Change_PlayerName
  (params (PlayerName%20 :type Text))
  (Variables|Default|SetPlayerProfile_info (Utilities|Struct|MakeS_Player_Profile PlayerName%20 (.charrowname (Variables|Default|GetPlayerProfile_info)) (.characterclass (Variables|Default|GetPlayerProfile_info))))
  (CallFunction|SaveProfile))

(event Custom|TravelToMap
  (params (NumConnectedPlayers :type Integer) (MapName :type String))
  (bind _output_get (Variables|Default|SetNum%20Connected%20Players NumConnectedPlayers))
  (Development|ExecuteConsoleCommand (Utilities|String|Append "servertravel " MapName) (Game|GetPlayerController _output_get)))

(fn UIShowMainMenu
  (bind _returnvalue (Game|GetPlayerController 0))
  (Utilities|IsValid (Variables|Default|GetWB_MainMenu)
    (:Is%20Valid
      _)
    (:Is%20Not%20Valid
      _))
  (bind _returnvalue_2 (UserInterface|CreateWidget "/Game/Widgets/startMenu.startMenu_C" _returnvalue))
  (Variables|Default|SetWB_MainMenu _returnvalue_2)
  (UserInterface|Viewport|AddtoViewport (Variables|Default|GetWB_MainMenu) 0)
  (Input|SetInputModeUIOnly _returnvalue 0 "DoNotLock")
  (Variables|/Script/Engine.PlayerController|SetbShowMouseCursor _returnvalue true)
  (CallFunction|CheckforSaveProfile)
  (Rendering|Components|TextRender|SetText (Variables|/Game/Widgets/startMenu.startMenu_C|GetInput_PlayerName (Variables|Default|GetWB_MainMenu)) (.PlayerName (Utilities|Struct|BreakS_Player_Profile (Variables|Default|GetPlayerProfile_info))))
  (return))

(fn CheckforSaveProfile
  (bind _returnvalue (SaveGame|DoesSaveGameExist (Variables|Default|GetPlayerProfile_slot)))
  (if _returnvalue
    (bind _assg_player_profile (CallFunction|LoadProfile))
    (Variables|Default|SetSG_PlayerProfile _assg_player_profile)
    (else
      (CallFunction|SaveProfile)))
  (return))

(fn LoadProfile
  (bind _returnvalue (SaveGame|LoadGamefromSlot (Variables|Default|GetPlayerProfile_slot)))
  (bind _assg_player_profile (Utilities|Casting|CastToSG_PlayerProfile _returnvalue))
  (Variables|Default|SetPlayerProfile_info (Variables|/Game/SaveData/SG_PlayerProfile.SG_PlayerProfile_C|GetplayerProfile _assg_player_profile))
  (return _assg_player_profile))

(fn SaveProfile
  (Utilities|IsValid (Variables|Default|GetSG_PlayerProfile)
    (:Is%20Valid
      (Variables|/Game/SaveData/SG_PlayerProfile.SG_PlayerProfile_C|SetplayerProfile (Variables|Default|GetSG_PlayerProfile) (Variables|Default|GetPlayerProfile_info))
      (SaveGame|SaveGametoSlot (Variables|Default|GetSG_PlayerProfile) (Variables|Default|GetPlayerProfile_slot))
      (return))
    (:Is%20Not%20Valid
      (bind _returnvalue (SaveGame|CreateSaveGameObject "/Game/SaveData/SG_PlayerProfile.SG_PlayerProfile_C"))
      (Variables|Default|SetSG_PlayerProfile _returnvalue))))

(fn UIShowMPMenu)