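; Lobby game mode that tracks connected menu controllers and shows each player as a character on a lobby spot.
; New players on the lobby maps get their menu and setup; logout destroys their character and frees the spot.
; UpdateLobby copies profiles into player states, then refreshes name lists and characters.
; Characters spawn on free spots and receive name, data-table mesh and animation through MC-prefixed calls, also used for single-player profile changes.
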(event Custom|UpdateLobby
  (params (PlayerNames :type Boolean) (CharacterSelect :type Boolean))
  (Utilities|Array|Clear (Variables|Default|GetAll_PlayersProfiles))
  (for (_array_element _array_index) (Variables|Default|GetAll_ConnetedPlayers)
    (Utilities|Array|SetArrayElem (Variables|Default|GetAll_PlayersProfiles) _array_index (Variables|/Game/FrameWorks/BP_GameMenu_Controller.BP_GameMenu_Controller_C|GetPlayerProfileInfo _array_element) true)
    (bind _asbp_game_player_state (Utilities|Casting|CastToBP_Game_PlayerState (Variables|/Script/Engine.Controller|GetPlayerState _array_element)))
    (Variables|/Game/FrameWorks/BP_Game_PlayerState.BP_Game_PlayerState_C|SetS_PlayerProfile _asbp_game_player_state (Variables|/Game/FrameWorks/BP_GameMenu_Controller.BP_GameMenu_Controller_C|GetPlayerProfileInfo _array_element)))
  (for (_array_element_2 _array_index_2) (Variables|Default|GetAll_ConnetedPlayers)
    (if PlayerNames
      (Default|UpdatePlayerNames _array_element_2 (Variables|Default|GetAll_PlayersProfiles)))
    (if CharacterSelect
      (CallFunction|UpdateSelectedCharacter _array_index_2))))

(event Custom|UpdateSelectedCharacter
  (params (PlayerIndex :type Integer))
  (bind _all_connetedplayers (Variables|Default|GetAll_ConnetedPlayers))
  (bind _all_playersprofiles (Variables|Default|GetAll_PlayersProfiles))
  (bind _output (Utilities|Array|Get(acopy) _all_connetedplayers PlayerIndex))
  (bind _output_2 (Utilities|Array|Get(acopy) _all_playersprofiles PlayerIndex))
  (if (== (Variables|/Game/FrameWorks/BP_GameMenu_Controller.BP_GameMenu_Controller_C|GetBP_LobbyCharacter (Utilities|Array|Get(acopy) (Variables|Default|GetAll_ConnetedPlayers) PlayerIndex)) 0)
    (bind _availableplayerspot (CallFunction|GetLobbyPlayerSpot))
    (Variables|/Game/Lobby/lobby_Player_Spot.lobby_Player_Spot_C|SetIsSpotUsed _availableplayerspot true)
    (bind _returnvalue (Game|SpawnActorfromClass "/Game/Lobby/BP_lobby_Character.BP_lobby_Character_C" (Transformation|GetActorTransform _availableplayerspot) "Undefined" 0 0))
    (Variables|/Game/FrameWorks/BP_GameMenu_Controller.BP_GameMenu_Controller_C|SetBP_LobbyCharacter _output _returnvalue)
    (Variables|/Game/FrameWorks/BP_GameMenu_Controller.BP_GameMenu_Controller_C|SetBP_LobbyPlayerSpot _output _availableplayerspot))
  (Default|MCSetPlayerName (Variables|/Game/FrameWorks/BP_GameMenu_Controller.BP_GameMenu_Controller_C|GetBP_LobbyCharacter (Utilities|Array|Get(acopy) (Variables|Default|GetAll_ConnetedPlayers) PlayerIndex)) (.playername _output_2))
  (bind _returnvalue_2 (Utilities|GetDataTableRow "/Game/NewPlayers/CharacterDataTable.CharacterDataTable" (.charrowname _output_2))
    (:then
      (Default|MCSetCharaMesh (Variables|/Game/FrameWorks/BP_GameMenu_Controller.BP_GameMenu_Controller_C|GetBP_LobbyCharacter (Utilities|Array|Get(acopy) (Variables|Default|GetAll_ConnetedPlayers) PlayerIndex)) (.CharactorMesh (Utilities|Struct|BreakS_CharaacterInfo _returnvalue_2)))
      (Default|MCPlayMeshAnim (Variables|/Game/FrameWorks/BP_GameMenu_Controller.BP_GameMenu_Controller_C|GetBP_LobbyCharacter (Utilities|Array|Get(acopy) (Variables|Default|GetAll_ConnetedPlayers) PlayerIndex)) (.LobbyAnimation (Utilities|Struct|BreakS_CharaacterInfo _returnvalue_2))))))

(event Custom|UpdateCharForController
  (params (Controller :type BP%20Game%20Menu%20Controller%20Object%20Reference) (PlayerProfile :type S%20Player%20Profile%20Structure))
  (bind _all_connetedplayers (Variables|Default|GetAll_ConnetedPlayers))
  (bind _returnvalue (Utilities|Array|FindItem _all_connetedplayers Controller))
  (Utilities|Array|SetArrayElem (Variables|Default|GetAll_PlayersProfiles) _returnvalue PlayerProfile true)
  (bind _asbp_game_player_state (Utilities|Casting|CastToBP_Game_PlayerState (Variables|/Script/Engine.Controller|GetPlayerState Controller)))
  (Variables|/Game/FrameWorks/BP_Game_PlayerState.BP_Game_PlayerState_C|SetS_PlayerProfile _asbp_game_player_state PlayerProfile)
  (CallFunction|UpdateSelectedCharacter _returnvalue))

(event EventBeginPlay)

(event EventTick
  (params (DeltaSeconds :type Float%20%28single-precision%29)))

(event EventHandleStartingNewPlayer
  (params (NewPlayer :type Player%20Controller%20Object%20Reference))
  (bind _returnvalue (Game|GetCurrentLevelName true))
  (switch string _returnvalue
    (:LobbyMenu_Map
      _)
    (:World2
      _))
  (bind _asbp_game_menu_controller (Utilities|Casting|CastToBP_GameMenu_Controller NewPlayer))
  (Utilities|Array|Add (Variables|Default|GetAll_ConnetedPlayers) _asbp_game_menu_controller)
  (Default|CreatLobbyMenu _asbp_game_menu_controller)
  (Default|InitialSetup _asbp_game_menu_controller))

(event EventOnLogout
  (params (ExitingController :type Controller%20Object%20Reference))
  (bind _asbp_game_menu_controller (Utilities|Casting|CastToBP_GameMenu_Controller ExitingController))
  (if (== (Variables|/Game/FrameWorks/BP_GameMenu_Controller.BP_GameMenu_Controller_C|GetBP_LobbyCharacter _asbp_game_menu_controller) 0)
    _
    (else
      (Actor|DestroyActor (Variables|/Game/FrameWorks/BP_GameMenu_Controller.BP_GameMenu_Controller_C|GetBP_LobbyCharacter _asbp_game_menu_controller))
      (Variables|/Game/Lobby/lobby_Player_Spot.lobby_Player_Spot_C|SetIsSpotUsed (Variables|/Game/FrameWorks/BP_GameMenu_Controller.BP_GameMenu_Controller_C|GetBP_LobbyPlayerSpot _asbp_game_menu_controller) false)))
  (Utilities|Array|RemoveItem (Variables|Default|GetAll_ConnetedPlayers) _asbp_game_menu_controller)
  (CallFunction|UpdateLobby true true))

(fn ConstructionScript)

(fn GetLobbyPlayerSpot
  (if (== (Utilities|Array|Length (Variables|Default|GetAllLobbPlayerSpots)) 0)
    (bind _outactors (Actor|GetAllActorsOfClass "/Game/Lobby/lobby_Player_Spot.lobby_Player_Spot_C"))
    (Variables|Default|SetAllLobbPlayerSpots _outactors))
  (bind _array_element (Utilities|Array|ForEachLoopwithBreak (Variables|Default|GetAllLobbPlayerSpots) :!label _label)
    (:LoopBody
      (if (not (Variables|/Game/Lobby/lobby_Player_Spot.lobby_Player_Spot_C|GetIsSpotUsed _array_element))
        (goto _label Break)))
    (:Completed
      (return _array_element))))