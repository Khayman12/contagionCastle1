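; AI rat pawn that hunts players in a game with human and Monster roles.
; On RatsAi possession it retries FindPlayer, meant to balance rats per player but succeeding only with one due to an inverted index check, then loops a chase.
; Sighting a pawn plays a sound for non-Monsters, triggers server-side pursuit and delayed random roaming.
; While Health is non-negative, Tick heals a Monster player 0 or damages other roles, regardless of distance.
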(event OnSeePawn(PawnSensing)
  (params (Pawn :type Pawn%20Object%20Reference))
  (Utilities|FlowControl|Sequence
    (:then_0
      (CallFunction|SqeekServer)
      (CallFunction|Sqeek)
      (if (Networking|IsServer)
        (CallFunction|Sqeekmulti)
        (Development|PrintString "seeing")
        (AI|AIMoveTo self "0, 0, 0" Pawn 5.0 false)
        (else
          (CallFunction|Sqeekmulti))))
    (:then_1
      (Utilities|FlowControl|RetriggerableDelay 0.5)
      (CallFunction|RandomRoam))))

(event Custom|sqeek
  (bind _asbp_base_player (Utilities|Casting|CastToBP_basePlayer (Game|Player|GetPlayerPawn 0)))
  (Development|PrintString (Utilities|String|ToString(Boolean) (or (== (Variables|/Game/NewPlayers/BP_basePlayer.BP_basePlayer_C|GetcharRowName _asbp_base_player) "Player1") (== (Variables|/Game/NewPlayers/BP_basePlayer.BP_basePlayer_C|GetcharRowName _asbp_base_player) "Player2"))))
  (if (not (== (Variables|/Game/NewPlayers/BP_basePlayer.BP_basePlayer_C|GetcharRowName _asbp_base_player) "Monster"))
    (Audio|PlaySoundatLocation "/Game/StarterContent/Audio/Explosion02.Explosion02" (Transformation|GetActorLocation) "0, 0, 0" 1.0 5.0 0.0 0 0 0 0)
    (if (== (Variables|/Game/NewPlayers/BP_basePlayer.BP_basePlayer_C|GetcharRowName _asbp_base_player) "Monster")
      (Audio|PlaySoundatLocation "/Game/StarterContent/Audio/Explosion02.Explosion02" (Transformation|GetActorLocation) "0, 0, 0" 1.0 5.0 0.0 0 0 0 0))))

(event Custom|sqeekmulti
  (bind _asbp_base_player (Utilities|Casting|CastToBP_basePlayer (Game|Player|GetPlayerPawn 0)))
  (Development|PrintString (Utilities|String|ToString(Boolean) (or (== (Variables|/Game/NewPlayers/BP_basePlayer.BP_basePlayer_C|GetcharRowName _asbp_base_player) "Player1") (== (Variables|/Game/NewPlayers/BP_basePlayer.BP_basePlayer_C|GetcharRowName _asbp_base_player) "Player2"))))
  (if (not (== (Variables|/Game/NewPlayers/BP_basePlayer.BP_basePlayer_C|GetcharRowName _asbp_base_player) "Monster"))
    (Audio|PlaySoundatLocation "/Game/StarterContent/Audio/Explosion02.Explosion02" (Transformation|GetActorLocation) "0, 0, 0" 1.0 5.0 0.0 0 0 0 0)
    (if (== (Variables|/Game/NewPlayers/BP_basePlayer.BP_basePlayer_C|GetcharRowName _asbp_base_player) "Monster")
      (Audio|PlaySoundatLocation "/Game/StarterContent/Audio/Explosion02.Explosion02" (Transformation|GetActorLocation) "0, 0, 0" 1.0 5.0 0.0 0 0 0 0))))

(event Custom|sqeekServer
  (bind _asbp_base_player (Utilities|Casting|CastToBP_basePlayer (Game|Player|GetPlayerPawn 0)))
  (Development|PrintString (Utilities|String|ToString(Boolean) (or (== (Variables|/Game/NewPlayers/BP_basePlayer.BP_basePlayer_C|GetcharRowName _asbp_base_player) "Player1") (== (Variables|/Game/NewPlayers/BP_basePlayer.BP_basePlayer_C|GetcharRowName _asbp_base_player) "Player2"))))
  (if (not (== (Variables|/Game/NewPlayers/BP_basePlayer.BP_basePlayer_C|GetcharRowName _asbp_base_player) "Monster"))
    (Audio|PlaySoundatLocation "/Game/StarterContent/Audio/Explosion02.Explosion02" (Transformation|GetActorLocation) "0, 0, 0" 1.0 5.0 0.0 0 0 0 0)
    (if (== (Variables|/Game/NewPlayers/BP_basePlayer.BP_basePlayer_C|GetcharRowName _asbp_base_player) "Monster")
      (Audio|PlaySoundatLocation "/Game/StarterContent/Audio/Explosion02.Explosion02" (Transformation|GetActorLocation) "0, 0, 0" 1.0 5.0 0.0 0 0 0 0))))

(event Custom|RandomRoam
  (AI|AIMoveTo self (.RandomLocation (AI|Navigation|GetRandomReachablePointinRadius (Transformation|GetActorLocation) 1.5e+03 0 0)) 0 5.0 false
    (:OnSuccess
      (CallFunction|RandomRoam))))

(event Custom|OnAISpawned
  (bind (_isvalidplayerfound1 _newplayer1) (CallFunction|FindPlayer :!label _label))
  (if _isvalidplayerfound1
    (Variables|Default|SetTargetPlayer _newplayer1)
    (CallFunction|MovetoPlayer)
    (else
      (Utilities|FlowControl|Delay 0.5)
      (goto _label))))

(event Custom|MoveToPlayer
  (if (Variables|Default|GetisAlive)
    (AI|AIMoveTo self "0, 0, 0" (Variables|Default|GetTargetPlayer) 1e+02 false
      (:OnSuccess
        _)
      (:OnFail
        _))
    (Utilities|FlowControl|Delay 2.0)
    (CallFunction|MovetoPlayer)))

(event EventBeginPlay)

(event EventPossessed
  (params (NewController :type Controller%20Object%20Reference))
  (bind _asrats_ai (Utilities|Casting|CastToRatsAi NewController))
  (Variables|Default|SetAs%20Rats%20Ai _asrats_ai)
  (CallFunction|OnAISpawned))

(event Game|Damage|EventAnyDamage
  (params (Damage :type Float%20%28single-precision%29) (DamageType :type Damage%20Type%20Object%20Reference) (InstigatedBy :type Controller%20Object%20Reference) (DamageCauser :type Actor%20Object%20Reference))
  (Variables|Default|Sethealth (- (Variables|Default|Gethealth) Damage)))

(event EventTick
  (params (DeltaSeconds :type Float%20%28single-precision%29))
  (if (>= (Variables|Default|Gethealth) 0.0)
    (bind _asbp_base_player (Utilities|Casting|CastToBP_basePlayer (Game|Player|GetPlayerPawn 0)))
    (if (== (Variables|/Game/NewPlayers/BP_basePlayer.BP_basePlayer_C|GetcharRowName _asbp_base_player) "Monster")
      (bind _asbp_monster (Utilities|Casting|CastToBP_Monster (Game|Player|GetPlayerPawn 0)))
      (Variables|/Game/NewPlayers/BP_basePlayer.BP_basePlayer_C|SetHealth _asbp_monster (+ (Variables|/Game/NewPlayers/BP_basePlayer.BP_basePlayer_C|GetHealth _asbp_monster) 5.0))
      (else
        (Game|Damage|ApplyDamage _asbp_base_player 1.0 0 0)))))

(fn ConstructionScript)

(fn FindPlayer
  (bind _outactors (Actor|GetAllActorsOfClass "/Game/NewPlayers/BP_basePlayer.BP_basePlayer_C"))
  (bind _output_get (LocalVariables|SetLcl_AllPlayer _outactors))
  (if (Utilities|Array|IsNotEmpty _output_get)
    (if (== (Utilities|Array|Length (LocalVariables|GetLcl_AllPlayer)) 1)
      (LocalVariables|Setlcl_isValidPlayerFound true)
      (LocalVariables|SetLcl_NewPlayer (Utilities|Array|Get(acopy) (LocalVariables|GetLcl_AllPlayer)))
      (else
        (for _array_element (LocalVariables|GetLcl_AllPlayer)
          (Utilities|Array|Add (LocalVariables|GetLcl_All_AIRats) (Variables|/Game/NewPlayers/BP_basePlayer.BP_basePlayer_C|GetNumAiRats _array_element)))
        (LocalVariables|SetLcl_lowestIndex (.IndexOfMinValue (Math|Integer|MinOfIntArray (LocalVariables|GetLcl_All_AIRats))))
        (if (== (LocalVariables|GetLcl_lowestIndex) -1)
          (Math|Integer|IncrementInt (Variables|/Game/NewPlayers/BP_basePlayer.BP_basePlayer_C|GetNumAiRats (Utilities|Array|Get(acopy) (LocalVariables|GetLcl_AllPlayer) (LocalVariables|GetLcl_lowestIndex)))
            (:%20%20
              (LocalVariables|SetLcl_NewPlayer (Utilities|Array|Get(acopy) (LocalVariables|GetLcl_AllPlayer) (LocalVariables|GetLcl_lowestIndex)))
              (LocalVariables|Setlcl_isValidPlayerFound true)))
          (else
            (LocalVariables|Setlcl_isValidPlayerFound false)))))
    (else
      (LocalVariables|Setlcl_isValidPlayerFound false)))
  (return (LocalVariables|Getlcl_isValidPlayerFound) (LocalVariables|GetLcl_NewPlayer)))